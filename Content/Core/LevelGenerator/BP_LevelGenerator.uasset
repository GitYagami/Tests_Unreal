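; Level generator actor that builds a continually growing row of building meshes along the Y axis from its XY position.
; On BeginPlay it caches the player, then loops through the buildings data table, async-loading meshes.
; Each becomes a runtime component with scaled-down row scale and a random material, advancing the offset by its Y bounds extent.
; A delay loops back to reread the table; SpawnBuildings is an empty stub.
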(event EventTick
  (params (DeltaSeconds :type Float%20%28single-precision%29)))

(event EventBeginPlay
  (bind _returnvalue (Transformation|GetActorLocation))
  (bind _dt_buildings (Variables|Default|GetDT_Buildings))
  (bind _datatable (Utilities|Struct|BreakDataTableRowHandle _dt_buildings))
  (bind _asbp_player (Utilities|Casting|CastToBP_Player (Game|Player|GetPlayerPawn 0)))
  (Variables|Default|SetBP_Player _asbp_player)
  (bind _outrownames (DataTable|GetDataTableRowNames _datatable :!label _label))
  (for _array_element _outrownames
    (bind _returnvalue_2 (Utilities|GetDataTableRow _datatable _array_element)
      (:then
        (Utilities|AsyncLoadAsset (.BuildingMesh (Utilities|Struct|BreakS_Buildings _returnvalue_2))
          (:then
            (bind _returnvalue_3 (AddComponent|AddStaticMeshComponent false))
            (Components|StaticMesh|SetStaticMesh _returnvalue_3 (Utilities|ResolveSoftReference (.BuildingMesh (Utilities|Struct|BreakS_Buildings _returnvalue_2))))
            (Transformation|SetWorldScale3D _returnvalue_3 (* (.scale (.BuildingTransform (Utilities|Struct|BreakS_Buildings _returnvalue_2))) 0.6))
            (Transformation|SetWorldLocation _returnvalue_3 (+ (Variables|Default|GetNewRelativeLocation) (Math|Vector|MakeVector (.x _returnvalue) (.y _returnvalue) 0.0)) false false)
            (Rendering|Material|CreateDynamicMaterialInstance _returnvalue_3 0 (.OutItem (Utilities|Array|Random (Variables|Default|GetMaterialArray))) "None" :!class /Script/Engine.PrimitiveComponent)
            (Variables|Default|SetNewRelativeLocation (+ (Variables|Default|GetNewRelativeLocation) (Math|Vector|MakeVector 0.0 (* (.Y (Math|Vector|BreakVector (.BoxExtent (Collision|GetComponentBounds _returnvalue_3)))) 1.0) 0.0)))
            (Utilities|FlowControl|Delay 2.0)
            (goto _label))))
      (:RowNotFound
        (Development|PrintString "ROW NOT FOUND")))))

(fn ConstructionScript)

(fn SpawnBuildings)