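; Enemy shooter that periodically turns toward the player and fires a projectile.
; Tick runs through a two-second Delay to throttle calls to Shoot.
; Shoot rotates the actor to face the player, then spawns BP_EnemyProjectile at FiringPoint, aimed at the player's location plus a distance-scaled velocity offset as simple lead aiming.
; Leftover player-cast and billboard "NextPosition" nodes are unused.
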(event Custom|Shoot
  (bind _returnvalue (Game|Player|GetPlayerPawn 0))
  (bind _firingpoint (Variables|Default|GetFiringPoint))
  (bind _returnvalue_2 (Transformation|GetActorLocation _returnvalue))
  (bind _returnvalue_3 (Transformation|GetWorldLocation _firingpoint))
  ;[1 1 1] Fonctionne mais c'est un peu la mort
  (Transformation|SetActorRotation (Math|Rotator|FindLookatRotation _returnvalue_3 _returnvalue_2))
  (Game|SpawnActorfromClass "/Game/Core/Enemies/BP_EnemyProjectile.BP_EnemyProjectile_C" (Math|Transform|MakeTransform _returnvalue_3 (Math|Rotator|FindLookatRotation _returnvalue_3 (+ _returnvalue_2 (* (/ (Transformation|GetDistanceTo 0) 1e+03) (Transformation|GetVelocity))))) "Undefined" "MultiplyWithRoot" 0 0))

(event EventBeginPlay)

(event EventTick
  (params (DeltaSeconds :type Float%20%28single-precision%29))
  (Utilities|FlowControl|Delay 2.0)
  (CallFunction|Shoot))

(fn ConstructionScript)