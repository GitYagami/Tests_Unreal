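; Enemy projectile Blueprint that reports player hits and signals when the player may instant-shield against it.
; Overlaps with the Player on the StartShield and EndShield components open and close the instant-shield window, which also starts closed on BeginPlay.
; A CollisionDamage overlap passes the projectile reference and location to the player pawn.
; All communication goes through messages to player pawn 0, leaving the response to the pawn.
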(event OnComponentBeginOverlap(StartShield)
  (params (OverlappedComponent :type Primitive%20Component%20Object%20Reference) (OtherActor :type Actor%20Object%20Reference) (OtherComp :type Primitive%20Component%20Object%20Reference) (OtherBodyIndex :type Integer) (bFromSweep :type Boolean) (SweepResult :type Hit%20Result%20Structure%20%28by%20ref%29))
  (if (Actor|ActorHasTag OtherActor "Player")
    (bind _output_get (Variables|Default|SetCanPlayerInstantShield true))
    (Class|BPItoPlayer|CanPlayerInstantShield(Message) (Game|Player|GetPlayerPawn 0) _output_get)))

(event OnComponentBeginOverlap(CollisionDamage)
  (params (OverlappedComponent :type Primitive%20Component%20Object%20Reference) (OtherActor :type Actor%20Object%20Reference) (OtherComp :type Primitive%20Component%20Object%20Reference) (OtherBodyIndex :type Integer) (bFromSweep :type Boolean) (SweepResult :type Hit%20Result%20Structure%20%28by%20ref%29))
  (if (Actor|ActorHasTag OtherActor "Player")
    (Class|BPItoPlayer|PlayerHitEnemyProjectile(Message) (Game|Player|GetPlayerPawn 0) self (Transformation|GetActorLocation))))

(event OnComponentBeginOverlap(EndShield)
  (params (OverlappedComponent :type Primitive%20Component%20Object%20Reference) (OtherActor :type Actor%20Object%20Reference) (OtherComp :type Primitive%20Component%20Object%20Reference) (OtherBodyIndex :type Integer) (bFromSweep :type Boolean) (SweepResult :type Hit%20Result%20Structure%20%28by%20ref%29))
  (if (Actor|ActorHasTag OtherActor "Player")
    (bind _output_get (Variables|Default|SetCanPlayerInstantShield false))
    (Class|BPItoPlayer|CanPlayerInstantShield(Message) (Game|Player|GetPlayerPawn 0) _output_get)))

(event EventBeginPlay
  (bind _output_get (Variables|Default|SetCanPlayerInstantShield false))
  (Class|BPItoPlayer|CanPlayerInstantShield(Message) (Game|Player|GetPlayerPawn 0) _output_get))

(fn ConstructionScript)