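; Configurable Chaos destructible actor that acts as a Blocker, optionally polarised, or a gatherable fluid Strain, optionally trapped.
; Construction builds the geometry collection, sets collision and material by type, and adds anchor placeholder shapes, plus InterpToMovement when mobile.
; BeginPlay swaps placeholders for anchor field actors and enables physics.
; Blockers notify the player on first overlap; breaking makes fragments overlap-only and releases anchors, while crumbling launches pieces upward.
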(event OnChaosCrumblingEvent(GeometryCollection)
  (params (CrumbleEvent :type Chaos%20Crumbling%20Event%20Structure%20%28by%20ref%29))
  (bind (_component _location _orientation _linearvelocity _angularvelocity _mass _localbounds _children) (Utilities|Struct|BreakChaosCrumblingEvent CrumbleEvent))
  (bind _asgeometry_collection_component (Utilities|Casting|CastToGeometryCollectionComponent _component))
  (for _array_element _children
    (Class|GeometryCollectionComponent|ApplyLinearVelocity _asgeometry_collection_component _array_element (Math|Vector|MakeVector 0.0 0.0 9999999.0))))

(event OnChaosBreakEvent(GeometryCollection)
  (params (BreakEvent :type Chaos%20Break%20Event%20Structure%20%28by%20ref%29))
  (Utilities|Array|AddUnique (Variables|Default|Gettestarray) (.location BreakEvent))
  (Utilities|Array|AddUnique (Variables|Default|Getarraytest) (.component BreakEvent))
  (switch Utilities|FlowControl|Switch|SwitchonE_DestructibleType (Variables|DestructibleType|GetDestructibleType)
    (:NewEnumerator0
      (Collision|SetCollisionResponsetoAllChannels (.component BreakEvent) "ECR_Overlap")
      (Collision|BindEventtoOnComponentBeginOverlap (.component BreakEvent) (delegate Custom|FragmentBeginOverlap))
      (Utilities|FlowControl|DoOnce false
        (:Completed
          (Class|GeometryCollectionComponent|RemoveAllAnchors (Variables|Default|GetGeometryCollection)))))))

(event Custom|FragmentBeginOverlap
  (params (OverlappedComponent :type Primitive%20Component%20Object%20Reference) (OtherActor :type Actor%20Object%20Reference) (OtherComp :type Primitive%20Component%20Object%20Reference) (OtherBodyIndex :type Integer) (bFromSweep :type Boolean) (SweepResult :type Hit%20Result%20Structure%20%28by%20ref%29))
  (if (Actor|ActorHasTag OtherActor "Player")
    _))

(event EventBeginPlay
  (|NotifiesGeometryCollectionEvents)
  (switch Utilities|FlowControl|Switch|SwitchonE_AnchorsType (Variables|Anchors|GetAnchorsType)
    (:NewEnumerator0
      (CallFunction|SpawnBoxAnchors))
    (:NewEnumerator1
      (CallFunction|SpawnSphereAnchors))))

(event EventSetCanStrainbeGathered
  (params (CanBeGathered? :type Boolean))
  (Variables|Default|SetHasBeenHit CanBeGathered?)
  (Variables|Default|SetCanBeGathered? CanBeGathered?))

(event OnComponentBeginOverlap(GeometryCollection)
  (params (OverlappedComponent :type Primitive%20Component%20Object%20Reference) (OtherActor :type Actor%20Object%20Reference) (OtherComp :type Primitive%20Component%20Object%20Reference) (OtherBodyIndex :type Integer) (bFromSweep :type Boolean) (SweepResult :type Hit%20Result%20Structure%20%28by%20ref%29))
  (bind _destructibletype (Variables|DestructibleType|GetDestructibleType))
  ;[0.15 0.15 0.15 0.5] PLAYER COLLISION
  (switch Utilities|FlowControl|Switch|SwitchonE_DestructibleType _destructibletype
    (:NewEnumerator0
      (if (and (Actor|ActorHasTag OtherActor "Player") (not (Variables|Default|GetAlreadyCollidedByPlayer?)))
        (Variables|Default|SetAlreadyCollidedByPlayer? true)
        (Class|BPItoPlayer|PlayerHitBlocker(Message) OtherActor self _destructibletype (Variables|DestructibleType|GetIsPolarised?) (Transformation|GetActorLocation))))))

(fn ConstructionScript
  (bind _geometrycollection (|AddGeometryCollection))
  (Rendering|SetRenderCustomDepth _geometrycollection true :!pinned true) ; Intègre le component dans le Custom Depth
  (|AddAnchorsbyType)
  (switch Utilities|FlowControl|Switch|SwitchonE_DestructibleType (Variables|DestructibleType|GetDestructibleType)
    (:NewEnumerator0
      (if (not (Variables|DestructibleType|GetIsPolarised?))
        (Collision|SetCollisionObjectType _geometrycollection "ECC_GameTraceChannel1")
        (Rendering|Material|SetMaterial (Variables|Default|GetGeometryCollection) 0 "/Game/Assets/Chaos/GeometryCollections/Materials/MI_Blocker.MI_Blocker")
        (else
          (Collision|SetCollisionObjectType _geometrycollection "ECC_GameTraceChannel11")
          (Rendering|Material|SetMaterial (Variables|Default|GetGeometryCollection) 0 "/Game/Assets/Chaos/GeometryCollections/Materials/MI_Blocker.MI_Blocker"))))
    (:NewEnumerator1
      (if (not (Variables|DestructibleType|GetIsTrapped?))
        (Collision|SetCollisionObjectType _geometrycollection "ECC_GameTraceChannel3")
        (Rendering|Material|CreateDynamicMaterialInstance (Variables|Default|GetGeometryCollection) 0 "/Game/Assets/Chaos/GeometryCollections/Materials/MI_Strain.MI_Strain" "None" :!class /Script/Engine.PrimitiveComponent)
        (CallFunction|AddWidgetComponent)
        (Collision|SetCollisionResponsetoChannel _geometrycollection "ECC_GameTraceChannel7" "ECR_Overlap")
        (else
          (Collision|SetCollisionObjectType _geometrycollection "ECC_GameTraceChannel10")
          (Rendering|Material|SetMaterial (Variables|Default|GetGeometryCollection) 0 "/Game/Assets/Chaos/GeometryCollections/Materials/MI_Strain.MI_Strain")))))
  (switch Utilities|FlowControl|Switch|SwitchonE_DestructibleMovementType (Variables|DestructibleType|GetDestructibleMovementType)
    (:NewEnumerator0
      (Utilities|Array|Clear (Variables|MobileGCVariables|GetTargetLocation)))
    (:NewEnumerator1
      (CallFunction|AddInterptoMovementComponent))
    (:NewEnumerator2
      (Utilities|Array|Clear (Variables|MobileGCVariables|GetTargetLocation)))))

(fn AddInterptoMovementComponent
  (bind _returnvalue (AddComponent|AddInterptoMovementComponent))
  (Utilities|IsValid _returnvalue
    (:Is%20Valid
      (Variables|/Script/Engine.InterpToMovementComponent|SetBehaviourType _returnvalue (Variables|MobileGCVariables|GetMovementType))
      (Class|InterptoMovementComponent|AddControlPointPosition _returnvalue "0, 0, 0" true)
      (for _array_element (Variables|MobileGCVariables|GetTargetLocation)
        (Class|InterptoMovementComponent|AddControlPointPosition _returnvalue _array_element true)
        (Variables|/Script/Engine.InterpToMovementComponent|SetDuration _returnvalue (Variables|MobileGCVariables|GetMovementDuration))))))

(fn SpawnBoxAnchors
  (bind _geometrycollection (Variables|Default|GetGeometryCollection))
  (for _array_element (Actor|GetComponentsByClass "/Script/Engine.BoxComponent")
    (bind _returnvalue (Game|SpawnActorfromClass "/Engine/EditorResources/FieldNodes/FS_AnchorField_Generic.FS_AnchorField_Generic_C" (Math|Transform|MakeTransform (Transformation|GetWorldLocation _array_element) "0, 0, 0" (Transformation|GetWorldScale _array_element)) "Undefined" "MultiplyWithRoot" 0 0))
    (Components|DestroyComponent _array_element)
    (Collision|SetActorEnableCollision _returnvalue false)
    (Utilities|Array|Add (Variables|/Script/GeometryCollectionEngine.GeometryCollectionComponent|GetInitializationFields _geometrycollection) _returnvalue)
    (Physics|SetSimulatePhysics _geometrycollection true)))

(fn SpawnSphereAnchors
  (bind _geometrycollection (Variables|Default|GetGeometryCollection))
  (for _array_element (Actor|GetComponentsByClass "/Script/Engine.SphereComponent")
    (bind _returnvalue (Game|SpawnActorfromClass "/Engine/EditorResources/FieldNodes/FS_AnchorField_Generic.FS_AnchorField_Generic_C" (Math|Transform|MakeTransform (Transformation|GetWorldLocation _array_element) "0, 0, 0" (Transformation|GetWorldScale _array_element)) "Undefined" "MultiplyWithRoot" 0 0))
    (Components|DestroyComponent _array_element)
    (Variables|/Engine/EditorResources/FieldNodes/FS_AnchorField_Generic.FS_AnchorField_Generic_C|SetAnchor%20Falloff%20Shape _returnvalue "NewEnumerator1")
    (Collision|SetActorEnableCollision _returnvalue false)
    (Utilities|Array|Add (Variables|/Script/GeometryCollectionEngine.GeometryCollectionComponent|GetInitializationFields _geometrycollection) _returnvalue)
    (Physics|SetSimulatePhysics _geometrycollection true)))

(fn AddWidgetComponent
  (bind _returnvalue (AddComponent|AddWidgetComponent false (Math|Transform|MakeTransform "0.000000,0.000000,50.000000" "0, 0, 0" "1.000000,1.000000,1.000000")))
  (UserInterface|SetWidget _returnvalue (Variables|Default|GetWidget))
  (Class|WidgetComponent|SetWidgetSpace _returnvalue "Screen")
  (Class|WidgetComponent|SetDrawatDesiredSize _returnvalue true)
  (Development|SetHiddeninGame _returnvalue true false))

(fn GetCanStrainbeGathered
  (return (Variables|Default|GetCanBeGathered?)))

(fn GetDestructibleInfo
  (return (Variables|DestructibleType|GetDestructibleType) (Variables|DestructibleType|GetDestructibleMovementType) (Variables|Default|GetHasBeenHit) (Variables|DestructibleType|GetIsPolarised?) (Variables|DestructibleType|GetIsTrapped?)))

(fn GetFluidAmountinStrain
  (return (Variables|Default|GetFluidAmountInStrain)))