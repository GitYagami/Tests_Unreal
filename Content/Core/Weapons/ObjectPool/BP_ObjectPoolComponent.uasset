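; Actor component that pools weapon-related actors for reuse instead of spawning them on demand.
; One second after BeginPlay, a delay that lets weapon velocity values initialize, it pre-spawns the pool with lifetime and right-weapon values, marking each actor unused.
; SpawnFromPool linearly searches for a free actor, applies the hold multiplier, moves it to SpawnTransform and marks it in use.
; It prints a debug message when no valid actor is found.
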(event Custom|InitializePool
  (for _index (range 0 (Variables|Default|GetPoolSize))
    (bind _returnvalue (Game|SpawnActorfromClass (Variables|Default|GetPooledActorClass) (Math|Transform|MakeTransform "0, 0, 0" "0, 0, 0" "1.000000,1.000000,1.000000") "Undefined" "MultiplyWithRoot" 0 (Variables|Default|GetTimeToLive) (Variables|Default|GetRightWeaponValues) 0))
    (Utilities|Array|AddUnique (Variables|Default|GetObjectPool) _returnvalue)
    (Default|SetinUse _returnvalue false)))

(event EventBeginPlay
  (Utilities|FlowControl|Delay 1.0) ; Obligé de faire ça pour que le RightWeaponVelocity ait le temps de s'initialiser avant que la Pool soit initialisé
  (CallFunction|InitializePool))

(event EventTick
  (params (DeltaSeconds :type Float%20%28single-precision%29)))

(fn FindFirstAvailableActor
  (for _array_element (Variables|Default|GetObjectPool)
    (if (not (Variables|/Game/Core/Weapons/ObjectPool/PooledActor.PooledActor_C|GetInUse _array_element))
      (return _array_element))))

(fn SpawnfromPool
  (params (SpawnTransform :type Transform) (HoldMultiplicator :type Float%20%28double-precision%29))
  (bind _pooledactor (CallFunction|FindFirstAvailableActor))
  (Utilities|IsValid _pooledactor
    (:Is%20Valid
      (Variables|/Game/Core/Weapons/ObjectPool/PooledActor.PooledActor_C|SetHoldMultiplicator _pooledactor HoldMultiplicator)
      (Transformation|SetActorTransform _pooledactor (Math|Transform|MakeTransform (.location SpawnTransform) (.rotation SpawnTransform) "1.000000,1.000000,1.000000"))
      (Default|SetinUse _pooledactor true)
      (return _pooledactor))
    (:Is%20Not%20Valid
      (Development|PrintString "Pooled Actor Invalid" true true "(R=1.000000,G=0.027276,B=0.000000,A=1.000000)"))))