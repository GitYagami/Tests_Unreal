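; Functional test that checks the player's left machine gun can hit a destructible actor.
; PrepareTest caches the player pawn as BP_Player.
; StartTest fires the weapon component's left machine gun line trace from the player camera with persistent debug drawing.
; It succeeds only if the blocking hit actor has the Destructible tag, and fails on a miss or any other hit.
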(event EventPrepareTest
  (bind _asbp_player (Utilities|Casting|CastToBP_Player (Game|Player|GetPlayerPawn 0)))
  (Variables|Default|SetBP_Player _asbp_player))

(event EventStartTest
  (bind _bp_player (Variables|Default|GetBP_Player))
  ;[1 0 0.9141] Test shooting sur un Destructible
  (bind _outhit (Default|ShootLeftMachineGunLineTrace (Variables|/Game/Core/Player/BP_Player.BP_Player_C|GetBP_WeaponComponent _bp_player) (Variables|/Game/Core/Player/BP_Player.BP_Player_C|GetCamera _bp_player) 0.0 "Persistent" 2e+03))
  (if (.bBlockingHit (Collision|BreakHitResult _outhit))
    (if (Actor|ActorHasTag (.HitActor (Collision|BreakHitResult _outhit)) "Destructible")
      (Class|FunctionalTest|FinishTest "Succeeded" "On a touché un Destructible 
 
 
")
      (else
        (Class|FunctionalTest|FinishTest "Failed" "N'a pas tiré")))
    (else
      (Class|FunctionalTest|FinishTest "Failed" "A tiré dans le vide"))))

(fn ConstructionScript)