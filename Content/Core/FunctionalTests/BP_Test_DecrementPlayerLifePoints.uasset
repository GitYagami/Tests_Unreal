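; Functional test Blueprint that exercises the player's life point decrement after damage.
; PrepareTest caches the player pawn as BP_Player, and StartTest handles only the Attack class, setting resistance and max life before calling UpdateLifePoints with damage scaled by resistance.
; The expected-value comparison is left unconnected and the branch condition is a constant true, so that path always reports success.
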(event EventPrepareTest
  (bind _asbp_player (Utilities|Casting|CastToBP_Player (Game|Player|GetPlayerPawn 0)))
  (Variables|Default|SetBP_Player _asbp_player))

(event EventStartTest
  (bind _bp_player (Variables|Default|GetBP_Player))
  (bind _player_values (Variables|/Game/Core/Player/BP_Player.BP_Player_C|GetPlayer%20Values _bp_player))
  (switch Utilities|FlowControl|Switch|SwitchonE_SelectedClass (Variables|/Game/Core/Player/BP_Player.BP_Player_C|GetE_SelectedClass _bp_player)
    (:NewEnumerator0
      (|SetBy-RefVar _player_values (Utilities|Struct|MakePlayerValues 0.8 1e+02 1.1 1.1))
      (bind _newcurrentlifepoints (Default|UpdateLifePoints _bp_player (* (Variables|/Game/Core/Player/BP_Player.BP_Player_C|GetDamages _bp_player) (Utilities|Struct|BreakPlayerValues _player_values))))
      (if true
        (Class|FunctionalTest|FinishTest "Succeeded" "Points de vie bien décrémentés.  
Attack = 88 PV 
 
 
")
        (else
          (Class|FunctionalTest|FinishTest "Failed" "Points de vie mal décrémentés"))))))

(fn ConstructionScript)