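; Functional test for player collision with a polarised blocker and the resulting life point loss.
; PrepareTest caches the player pawn, then StartTest requires its collision flag to be set and its life points to differ from 100.
; It then applies damage itself through UpdateLifePoints, passing if the new value does not exceed the maximum.
; An unconnected machine-gun line trace check for Destructible actors never runs.
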(event EventPrepareTest
  (bind _asbp_player (Utilities|Casting|CastToBP_Player (Game|Player|GetPlayerPawn 0)))
  (Variables|Default|SetBP_Player _asbp_player))

(event EventStartTest
  (bind _bp_player (Variables|Default|GetBP_Player))
  ;[0.5937 1 0] Test Collision + Points de vie
  (if (Variables|/Game/Core/Player/BP_Player.BP_Player_C|GetFT_IsColliding _bp_player)
    (if (not (== (Variables|/Game/Core/Player/BP_Player.BP_Player_C|GetCurrentLifePoints _bp_player) 1e+02))
      (bind (_newcurrentlifepoints _newmaxlifepoints) (Default|UpdateLifePoints (Variables|Default|GetBP_Player) -2e+01))
      (if (<= _newcurrentlifepoints _newmaxlifepoints)
        (Class|FunctionalTest|FinishTest "Succeeded" "Collision détectée 
+ 
Points de vie décrémentés 
 
 
")
        (else
          (Class|FunctionalTest|FinishTest "Failed" "Points de vie non décrémentés")))
      (else
        (Class|FunctionalTest|FinishTest "Failed" "Points de vie = 100")))
    (else
      (Class|FunctionalTest|FinishTest "Failed" "Collision Echouée"))))

(fn ConstructionScript)