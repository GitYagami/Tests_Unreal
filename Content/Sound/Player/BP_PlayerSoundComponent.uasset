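; Player sound component that plays Wwise audio for ship collisions, ship improvement, fluid fill and left and right weapon fire.
; Each event receives gameplay state and posts an AkEvent, with switches selecting destructible type, polarised or trapped variants.
; RTPCs feed machine-gun heat and right-projectile velocity into the shot sounds.
; Movement sound is marked non-functional, laser cannon only prints debug text, and right-shot charging plays nothing.
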(event Custom|SFX_PlayerCollisionSound
  (params (DestructibleType :type E_DestructibleType%20Enum :default "NewEnumerator0") (IsPolarised? :type Boolean) (Actor :type Actor%20Object%20Reference) (DestructibleLocation :type Vector))
  ;[0.15 0.15 0.15 0.5 40] COLLISION PLAYER / DESTRUCTIBLE
  (switch Utilities|FlowControl|Switch|SwitchonE_DestructibleType DestructibleType
    (:NewEnumerator0
      (if IsPolarised? ; S'il est polarisé, alors on joue ce son, sinon un autre
        (Class|AkGameplayStatics|SetSwitch "/Game/WwiseAudio/Switches/Default_Work_Unit/E_Destructible/E_Destructible-Blocker_Polarised.E_Destructible-Blocker_Polarised" Actor)
        (Class|AkGameplayStatics|PostEvent "/Game/WwiseAudio/Events/Default_Work_Unit/SFX_PlayerCollision.SFX_PlayerCollision" Actor)
        (else
          (Class|AkGameplayStatics|SetSwitch "/Game/WwiseAudio/Switches/Default_Work_Unit/E_Destructible/E_Destructible-Blocker.E_Destructible-Blocker" Actor)
          (Class|AkGameplayStatics|PostEvent "/Game/WwiseAudio/Events/Default_Work_Unit/SFX_PlayerCollision.SFX_PlayerCollision" Actor))))))

(event Custom|SFX_WeaponCollisionSound
  (params (DestructibleType :type E_DestructibleType%20Enum :default "NewEnumerator0") (IsPolarised? :type Boolean) (IsTrapped? :type Boolean) (Actor :type Actor%20Object%20Reference) (DestructibleLocation :type Vector))
  ;[0.15 0.15 0.15 0.5 40] COLLISION WEAPON / DESTRUCTIBLE
  (switch Utilities|FlowControl|Switch|SwitchonE_DestructibleType DestructibleType
    (:NewEnumerator0
      (if IsPolarised?
        (Class|AkGameplayStatics|SetSwitch "/Game/WwiseAudio/Switches/Default_Work_Unit/E_Destructible/E_Destructible-Blocker_Polarised.E_Destructible-Blocker_Polarised" Actor)
        (Class|AkGameplayStatics|PostEvent "/Game/WwiseAudio/Events/Default_Work_Unit/SFX_WeaponCollisionSound.SFX_WeaponCollisionSound" Actor)
        (else
          (Class|AkGameplayStatics|SetSwitch "/Game/WwiseAudio/Switches/Default_Work_Unit/E_Destructible/E_Destructible-Blocker.E_Destructible-Blocker" Actor)
          (Class|AkGameplayStatics|PostEvent "/Game/WwiseAudio/Events/Default_Work_Unit/SFX_WeaponCollisionSound.SFX_WeaponCollisionSound" Actor))))
    (:NewEnumerator1
      (if IsTrapped?
        (Class|AkGameplayStatics|SetSwitch "/Game/WwiseAudio/Switches/Default_Work_Unit/E_Destructible/E_Destructible-Strain_Trapped.E_Destructible-Strain_Trapped" Actor)
        (Class|AkGameplayStatics|PostEvent "/Game/WwiseAudio/Events/Default_Work_Unit/SFX_WeaponCollisionSound.SFX_WeaponCollisionSound" Actor)
        (else
          (Class|AkGameplayStatics|SetSwitch "/Game/WwiseAudio/Switches/Default_Work_Unit/E_Destructible/E_Destructible-Strain.E_Destructible-Strain" Actor)
          (Class|AkGameplayStatics|PostEvent "/Game/WwiseAudio/Events/Default_Work_Unit/SFX_WeaponCollisionSound.SFX_WeaponCollisionSound" Actor))))))

(event Custom|SFX_PlayerMovementSound
  (params (PlayerSpeed :type Float%20%28double-precision%29))
  ;[0.15 0.15 0.15 0.5 40] PLAYER IMPROVE
  ;;[1 0.008842 0 0.5] NON FONCTIONNEL
  (Audio|PlaySound2D 0 1.0 1.0 0.0 0 0))

(event Custom|SFX_ImproveNotPossible
  ;[0.15 0.15 0.15 0.5 40] PLAYER IMPROVE
  (Class|AkGameplayStatics|PostEvent "/Game/WwiseAudio/Events/Default_Work_Unit/SFX_ImproveNotPossible.SFX_ImproveNotPossible"))

(event Custom|SFX_PlayerImproveSound
  (params (ImproveCount :type Integer) (PlayerSpeed :type Float%20%28double-precision%29))
  ;[0.15 0.15 0.15 0.5 40] PLAYER IMPROVE
  (Class|AkGameplayStatics|PostEvent "/Game/WwiseAudio/Events/Default_Work_Unit/SFX_PlayerImprove.SFX_PlayerImprove"))

(event Custom|SFX_FluidAmountIncreasingSound
  (params (CurrentFluidAmount :type Float%20%28double-precision%29) (MaxFluidAmount :type Float%20%28double-precision%29))
  ;[0.15 0.15 0.15 0.5 40] FLUID AMOUNT
  (if (not (>= CurrentFluidAmount MaxFluidAmount)) ; Si on est aux max du fluide, alors on fait rien (TRUE). \nSinon on joue le son de Fluide qui augmente (FALSE)
    (Class|AkGameplayStatics|PostEvent "/Game/WwiseAudio/Events/Default_Work_Unit/SFX_FluidFill.SFX_FluidFill")))

(event Custom|SFX_MaxFluidAmountSound
  ;[0.15 0.15 0.15 0.5 40] FLUID AMOUNT
  (Class|AkGameplayStatics|PostEvent "/Game/WwiseAudio/Events/Default_Work_Unit/SFX_FluidFilled.SFX_FluidFilled"))

(event Custom|SFX_ShootLeft_LaserCannon
  (params (HeatValue :type Float%20%28double-precision%29) (LaserCannonChargingValue :type Float%20%28double-precision%29))
  (if (> HeatValue LaserCannonChargingValue) ; Vérifie si tu dépasses la ChargingValue\nTRUE = Tu dépasses, donc ta barre change de couleur\nFALSE = Tu es en trains de charger le canon
    (Development|PrintString "TRUE" false true "(R=1.000000,G=0.186766,B=0.000000,A=1.000000)" 0.1)
    (else
      (Development|PrintString "FALSE" false true "(R=1.000000,G=0.378933,B=0.000000,A=1.000000)" 3.0))))

(event Custom|SFX_ShootLeft_MachineGun
  (params (HeatValue :type Float%20%28double-precision%29))
  (Class|AkGameplayStatics|SetRTPCValue "/Game/WwiseAudio/Game_Parameters/Default_Work_Unit/Overheat_Level.Overheat_Level" HeatValue)
  (Class|AkGameplayStatics|PostEvent "/Game/WwiseAudio/Events/Default_Work_Unit/SFX_CanonShot.SFX_CanonShot"))

(event Custom|SFX_ShootRightSound
  (params (FinalHoldMultiplicator :type Float%20%28double-precision%29) (RightWeaponVelocity :type Float%20%28double-precision%29))
  (Class|AkGameplayStatics|SetRTPCValue "/Game/WwiseAudio/Game_Parameters/Default_Work_Unit/Projectil_Velocity.Projectil_Velocity" RightWeaponVelocity)
  (Class|AkGameplayStatics|PostEvent "/Game/WwiseAudio/Events/Default_Work_Unit/SFX_PolarisedShot.SFX_PolarisedShot"))

(event Custom|SFX_ShootRightLoadingSound
  (params (HoldMultiplicator :type Float%20%28double-precision%29) (IsVisible :type Boolean))
  (if IsVisible
    _))