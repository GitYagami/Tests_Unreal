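; BP_MainMenuHUD is the main menu HUD, which creates the widgets manager on BeginPlay, shows the cursor and focuses the main menu.
; Play hides the main menu and runs a sped-up level sequence cinematic, switching the widget switcher to the start run menu when it stops.
; Returning plays the same sequence in reverse, then restores the main menu.
; The Options event switches straight to the options menu.
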(event Custom|CE_MainMenuPlayBtnClicked
  ;[1 0 0.9141] PLAY BUTTON
  (Widget|SetVisibility (Variables|/Game/HUD/MainMenu/WBP_MainMenuWidgetsManager.WBP_MainMenuWidgetsManager_C|GetWBP_MainMenu (Variables|Default|GetWBP_MainMenuWidgetsManager)) "Hidden")
  (bind (_outactor _returnvalue) (Sequencer|Player|CreateLevelSequencePlayer "/Game/HUD/MainMenu/MainMenuToRunMenuCinematic.MainMenuToRunMenuCinematic" (Utilities|Struct|MakeMovieSceneSequencePlaybackSettings false "(Value=0)" "(TickIntervalSeconds=0.000000,EvaluationBudgetMicroseconds=0.000000,bTickWhenPaused=False,bAllowRounding=True)" 3.0 0.0 false false false false false false "ForceKeepState" false)))
  (Variables|Default|SetMainMenuToRunMenuSequence _outactor)
  (Sequencer|Player|Play (Variables|/Script/LevelSequence.LevelSequenceActor|GetSequencePlayer (Variables|Default|GetMainMenuToRunMenuSequence)) :!class /Script/MovieScene.MovieSceneSequencePlayer)
  (EventDispatchers|BindEventtoOnStop _returnvalue (delegate Custom|CE_LevelSequenceEnd)))

(event Custom|CE_OptionsMenuBtnClicked
  (bind _wbp_mainmenuwidgetsmanager (Variables|Default|GetWBP_MainMenuWidgetsManager))
  ;[0 1 0.7656] OPTIONS BUTTON
  (Class|WidgetSwitcher|SetActiveWidget (Variables|/Game/HUD/MainMenu/WBP_MainMenuWidgetsManager.WBP_MainMenuWidgetsManager_C|GetWidgetSwitcher _wbp_mainmenuwidgetsmanager) (Variables|/Game/HUD/MainMenu/WBP_MainMenuWidgetsManager.WBP_MainMenuWidgetsManager_C|GetWBP_OptionsMenu _wbp_mainmenuwidgetsmanager)))

(event Custom|CE_ReturnToMainMenu
  (bind _mainmenutorunmenusequence (Variables|Default|GetMainMenuToRunMenuSequence))
  (bind _sequenceplayer (Variables|/Script/LevelSequence.LevelSequenceActor|GetSequencePlayer _mainmenutorunmenusequence))
  (Widget|SetVisibility (Variables|/Game/HUD/MainMenu/WBP_MainMenuWidgetsManager.WBP_MainMenuWidgetsManager_C|GetWBP_StartRunMenu (Variables|Default|GetWBP_MainMenuWidgetsManager)) "Hidden")
  (Class|MovieSceneSequencePlayer|PlayReverse _sequenceplayer)
  (EventDispatchers|BindEventtoOnStop _sequenceplayer (delegate Custom|CE_ReversedLevelSequanceStop)))

(event Custom|CE_LevelSequenceEnd
  (bind _wbp_mainmenuwidgetsmanager (Variables|Default|GetWBP_MainMenuWidgetsManager))
  (bind _wbp_startrunmenu (Variables|/Game/HUD/MainMenu/WBP_MainMenuWidgetsManager.WBP_MainMenuWidgetsManager_C|GetWBP_StartRunMenu _wbp_mainmenuwidgetsmanager))
  ;[1 0 0.9141] PLAY BUTTON
  (Class|WidgetSwitcher|SetActiveWidget (Variables|/Game/HUD/MainMenu/WBP_MainMenuWidgetsManager.WBP_MainMenuWidgetsManager_C|GetWidgetSwitcher _wbp_mainmenuwidgetsmanager) _wbp_startrunmenu)
  (Widget|SetVisibility _wbp_startrunmenu "Visible"))

(event Custom|CE_ReversedLevelSequanceStop
  (bind _wbp_mainmenuwidgetsmanager (Variables|Default|GetWBP_MainMenuWidgetsManager))
  (bind _wbp_mainmenu (Variables|/Game/HUD/MainMenu/WBP_MainMenuWidgetsManager.WBP_MainMenuWidgetsManager_C|GetWBP_MainMenu _wbp_mainmenuwidgetsmanager))
  (Class|WidgetSwitcher|SetActiveWidget (Variables|/Game/HUD/MainMenu/WBP_MainMenuWidgetsManager.WBP_MainMenuWidgetsManager_C|GetWidgetSwitcher _wbp_mainmenuwidgetsmanager) _wbp_mainmenu)
  (Widget|SetVisibility _wbp_mainmenu "Visible"))

(event EventBeginPlay
  ;[0.5937 1 0] INIT
  (CallFunction|Init))

(fn ConstructionScript)

(fn Init
  (bind _returnvalue (Game|GetPlayerController 0))
  (bind _asbp_game_instance (Utilities|Casting|CastToBP_GameInstance (Game|GetGameInstance)))
  (Variables|Default|SetBP_GameInstance _asbp_game_instance)
  (bind _returnvalue_2 (UserInterface|CreateWidget "/Game/HUD/MainMenu/WBP_MainMenuWidgetsManager.WBP_MainMenuWidgetsManager_C" _returnvalue))
  (Variables|Default|SetWBP_MainMenuWidgetsManager _returnvalue_2)
  (UserInterface|Viewport|AddtoViewport _returnvalue_2 0)
  (Variables|/Script/Engine.PlayerController|SetbShowMouseCursor _returnvalue true)
  (Input|SetInputModeGameandUI _returnvalue (Variables|/Game/HUD/MainMenu/WBP_MainMenuWidgetsManager.WBP_MainMenuWidgetsManager_C|GetWBP_MainMenu (Variables|Default|GetWBP_MainMenuWidgetsManager)) "DoNotLock" true false))