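; In-game HUD that creates the widget manager, switches between game interface and menu screens, and updates player bars.
; On BeginPlay it caches class and weapon choices from the GameInstance; the switches on them are still empty.
; SetActiveWidget sets pause, cursor and input mode, while show events record HUD state in the GameInstance; the pause menu event is unwired.
; Update events drive life, fluid, hold and heat bars, recoloring heat for the Laser Cannon.
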(event EventBeginPlay
  (bind _asbp_game_instance (Utilities|Casting|CastToBP_GameInstance (Game|GetGameInstance)))
  (bind _output_get (Variables|Default|SetBP_GameInstance _asbp_game_instance))
  (bind (_leftweaponvalues _playervalues _rightweaponvalues _selectedclass _leftweapontype _rightweapontype) (Class|BPItoGameInstance|GetClassValues(Message) _output_get)) ; Ca permettra de changer des trucs dans l'interface en fonction de la classe / arme choisie
  (Variables|Default|SetSelected%20Class _selectedclass)
  (Variables|Default|SetLeft%20Weapon%20Type _leftweapontype)
  (Variables|Default|SetRight%20Weapon%20Type _rightweapontype)
  (bind _returnvalue (UserInterface|CreateWidget "/Game/HUD/InGame/WBP_InGameWidgetsManager.WBP_InGameWidgetsManager_C"))
  (bind _output_get_2 (Variables|Default|SetWBP_WidgetsManager _returnvalue))
  (Variables|Default|SetWBP_PlayerInterface (Variables|/Game/HUD/InGame/WBP_InGameWidgetsManager.WBP_InGameWidgetsManager_C|GetWBP_InGamePlayerInterface _output_get_2))
  (UserInterface|Viewport|AddtoViewport _output_get_2 0)
  (Utilities|FlowControl|Sequence
    (:then_0
      (switch Utilities|FlowControl|Switch|SwitchonE_RightWeaponType (Variables|Default|GetRight%20Weapon%20Type)))
    (:then_1
      (switch Utilities|FlowControl|Switch|SwitchonE_LeftWeaponType (Variables|Default|GetLeft%20Weapon%20Type)))
    (:then_2
      (switch Utilities|FlowControl|Switch|SwitchonE_SelectedClass (Variables|Default|GetSelected%20Class)))))

(event Custom|CE_ShowInGamePauseMenu
  ;[0 0.8359 1 1 50] SHOW PAUSE MENU
)

(event Custom|CE_ShowInGamePlayerInterface
  ;[1 0.8438 0 1 50] SHOW PLAYER INTERFACE
  (CallFunction|SetActiveWidget 0 false)
  (Variables|/Game/Core/BP_GameInstance.BP_GameInstance_C|SetHUD%20States (Variables|Default|GetBP_GameInstance) "NewEnumerator1"))

(event Custom|CE_ShowInGameOptionsMenu
  ;[1 0 0.5156 1 50] SHOW OPTIONS MENU
  (CallFunction|SetActiveWidget 2 true)
  (Variables|/Game/Core/BP_GameInstance.BP_GameInstance_C|SetHUD%20States (Variables|Default|GetBP_GameInstance) "NewEnumerator2"))

(event Custom|CE_ShowMainMenu
  ;[0 1 0.2031 1 50] SHOW MAIN MENU
  (CallFunction|SetActiveWidget 3 true)
  (Variables|/Game/Core/BP_GameInstance.BP_GameInstance_C|SetHUD%20States (Variables|Default|GetBP_GameInstance) "NewEnumerator0"))

(event Custom|CE_UpdatePlayerLifePoints
  (params (CurrentLifePoints :type Float%20%28double-precision%29) (MaxLifePoints :type Float%20%28double-precision%29))
  ;[0.125 0 1 1 40] UPDATE PLAYER LIFE POINTS
  (Progress|SetPercent (Variables|/Game/HUD/InGame/WBP_InGamePlayerInterface.WBP_InGamePlayerInterface_C|GetLifeBar (Variables|Default|GetWBP_PlayerInterface)) (/ CurrentLifePoints 1e+02)))

(event Custom|CE_UpdateHeatBar
  (params (HeatValue :type Float%20%28double-precision%29) (LaserCannonChargingValue :type Float%20%28double-precision%29))
  (bind _wbp_playerinterface (Variables|Default|GetWBP_PlayerInterface))
  (bind _heatbar (Variables|/Game/HUD/InGame/WBP_InGamePlayerInterface.WBP_InGamePlayerInterface_C|GetHeatBar _wbp_playerinterface))
  ;[1 0.4453 0 1 40] UPDATE HEATBAR
  (switch Utilities|FlowControl|Switch|SwitchonE_LeftWeaponType (Variables|Default|GetLeft%20Weapon%20Type)
    (:NewEnumerator0
      _)
    (:NewEnumerator1
      (if (> HeatValue LaserCannonChargingValue)
        (Class|ProgressBar|SetFillColorandOpacity _heatbar "(R=1.000000,G=0.533423,B=0.000000,A=1.000000)")
        (else
          (Class|ProgressBar|SetFillColorandOpacity _heatbar "(R=0.000000,G=0.619439,B=1.000000,A=1.000000)")))))
  (Progress|SetPercent (Variables|/Game/HUD/InGame/WBP_InGamePlayerInterface.WBP_InGamePlayerInterface_C|GetHeatBar (Variables|Default|GetWBP_PlayerInterface)) (/ HeatValue 1e+01)))

(event Custom|CE_UpdateFluidBar
  (params (CurrentFluidAmount :type Float%20%28double-precision%29) (MaxFluidAmount :type Float%20%28double-precision%29))
  ;[0.1953 1 0 1 40] UPDATE FLUID BAR
  (Progress|SetPercent (Variables|/Game/HUD/InGame/WBP_InGamePlayerInterface.WBP_InGamePlayerInterface_C|GetFluidBar (Variables|Default|GetWBP_PlayerInterface)) CurrentFluidAmount))

(event Custom|CE_UpdateHoldBar
  (params (HoldTime :type Float%20%28double-precision%29) (IsVisible? :type Boolean))
  (bind _wbp_playerinterface (Variables|Default|GetWBP_PlayerInterface))
  (bind _holdbar (Variables|/Game/HUD/InGame/WBP_InGamePlayerInterface.WBP_InGamePlayerInterface_C|GetHoldBar _wbp_playerinterface))
  ;[0 0.03906 1 1 40] UPDATE HOLD BAR
  (if IsVisible?
    (Widget|SetVisibility _holdbar "Visible")
    (Progress|SetPercent _holdbar HoldTime)
    (else
      (Widget|SetVisibility _holdbar "Hidden"))))

(fn ConstructionScript)

(fn SetActiveWidget
  (params (WidgetSwitcherIndex :type Integer) (bGamePaused? :type Boolean))
  (bind _returnvalue (Game|GetPlayerController 0))
  (Class|WidgetSwitcher|SetActiveWidgetIndex (Variables|/Game/HUD/InGame/WBP_InGameWidgetsManager.WBP_InGameWidgetsManager_C|GetWidgetSwitcher (Variables|Default|GetWBP_WidgetsManager)) WidgetSwitcherIndex)
  (Game|SetGamePaused bGamePaused?)
  (Utilities|IsValid _returnvalue
    (:Is%20Valid
      (Variables|/Script/Engine.PlayerController|SetbShowMouseCursor _returnvalue bGamePaused?)
      (if (not bGamePaused?)
        (Input|SetInputModeGameOnly _returnvalue false)
        (else
          (Input|SetInputModeGameandUI _returnvalue 0 "DoNotLock" true false))))))